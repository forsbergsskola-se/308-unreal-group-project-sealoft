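; Lantern Blueprint with a spot light that switches on according to the game's time.
; BeginPlay caches the BP_GameMode reference.
; Every Tick compares that game mode's Time with LampTurnOnTime, setting the light's intensity to zero at or before the threshold and to a fixed brightness after it.
; The switch is instant, with no fade, and intensity is rewritten each frame.
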(event `self.ReceiveTick`
  (params (DeltaSeconds :type "Float (single-precision)"))
  (if (<= (`/Game/BluePrints/BP_GameMode.Time` (stale `self.ReceiveBeginPlay` _asbp_game_mode)) (`self.LampTurnOnTime`))
    (`LightComponent.SetIntensity` (`self.SpotLight`) 0.0)
    (else
      (`LightComponent.SetIntensity` (`self.SpotLight`) 115.0))))

(event `self.ReceiveBeginPlay`
  (bind _asbp_game_mode (cast `/Game/BluePrints/BP_GameMode` (`GameplayStatics.GetGameMode`))))

(fn `UserConstructionScript`)