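; BP_BaseNpc is a base NPC that follows a timed route and offers dialogue, fetch quests and a shop.
; It AI-moves through WalkPoints, polling game-mode Time to advance and flagging shop positions on arrival.
; Interaction toggles both characters' movement and the UI, opening the shop at shop positions unless the player holds the quest item.
; Dialogue shows random lines, occasionally assigns item quests and pays coins on delivery.
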(event `self.ReceiveBeginPlay`
  (bind _walkpoints (`self.WalkPoints`))
  (bind (_output_walkpoint _output_pausetime _output_isshopposition) (break `/Game/BluePrints/WalkPoint` (`|GetArrayItem` (`self.WalkPoints`))))
  ;[1 1 1] AI Movement
  (if (not (<= (`KismetArrayLibrary.Array_Length` _walkpoints) 0)) :!label _label
    (`|AIMoveTo` self (0.0 0.0 0.0) _output_walkpoint 1.0
      (:`then`
        (bind _asbp_game_mode (cast `/Game/BluePrints/BP_GameMode` (`GameplayStatics.GetGameMode`)))
        (if (<= (`/Game/BluePrints/BP_GameMode.Time` _asbp_game_mode) _output_pausetime) :!label _label_2
          (`KismetSystemLibrary.Delay` 1.0)
          (goto _label_2)
          (else
            (`KismetArrayLibrary.Array_Remove` _walkpoints)
            (goto _label))))
      (:`OnSuccess`
        (set `self.IsInShop` _output_isshopposition)
        (`self.K2_SetActorRotation` (`self.K2_GetActorRotation` _output_walkpoint))))))

(event `/Game/BluePrints/IInteractable.On Interacted With`
  (params (Player :type "/Game/BluePrints/BP_Player Object Reference"))
  (bind _returnvalue (`GameplayStatics.GetPlayerController` 0))
  (bind _shopitems (`self.ShopItems`))
  (bind _helditem (`/Game/BluePrints/BP_Player.HeldItem` Player))
  (bind _charactermovement (`Character.CharacterMovement` Player))
  (bind _talktext (`/Game/BluePrints/WB_Dialouge.TalkText` (`self.UI`)))
  ;[1 1 1] Dialogue
  (bind _isa (`/Engine/EditorBlueprintResources/StandardMacros.FlipFlop`)
    (:`A`
      _)
    (:`B`
      _))
  (bind _output_get (set `self.IsInteracting` (not _isa)))
  (if _output_get
    (`CharacterMovementComponent.SetMovementMode` _charactermovement "MOVE_Walking" 0)
    (`CharacterMovementComponent.SetMovementMode` (`self.CharacterMovement`) "MOVE_Walking" 0)
    (bind _ui (`self.UI`)
      (:`then`
        (`Widget.SetVisibility` _ui "Hidden"))
      (:`else`
        _))
    (bind _shopui (`self.ShopUI`)
      (:`then`
        (`Widget.SetVisibility` _shopui "Hidden")
        (set `PlayerController.bShowMouseCursor` false (`GameplayStatics.GetPlayerController` 0)))
      (:`else`))
    (else
      (`CharacterMovementComponent.DisableMovement` _charactermovement)
      (`CharacterMovementComponent.DisableMovement` (`self.CharacterMovement`))
      (if (`self.IsInShop`)
        (bind _currentquest (`self.CurrentQuest`)
          (:`then`
            (if (== (`GameplayStatics.GetObjectClass` (`/Game/BluePrints/BP_Player.HeldItem` Player)) _currentquest)
              (`self.UI` :!label _label_3
                (:`then`
                  (`Widget.SetVisibility` (`self.UI`) "Visible"))
                (:`else`
                  (bind _returnvalue_2 (`|CreateWidget` "/Game/BluePrints/WB_Dialouge.WB_Dialouge_C" (`GameplayStatics.GetPlayerController` 0)))
                  (bind _output_get_2 (set `self.UI` _returnvalue_2))
                  (`UserWidget.AddToViewport` (`self.UI`) 0)
                  (`UserWidget.AddToViewport` _output_get_2 0)))
              (`self.CurrentQuest`
                (:`then`
                  (if (== (`GameplayStatics.GetObjectClass` _helditem) (`self.CurrentQuest`))
                    (bind _asbp_game_mode (cast `/Game/BluePrints/BP_GameMode` (`GameplayStatics.GetGameMode`)))
                    (set `/Game/BluePrints/BP_GameMode.Coins` (+ 100 (`/Game/BluePrints/BP_GameMode.Coins` _asbp_game_mode)) _asbp_game_mode)
                    (`TextBlock.SetText` _talktext "Thanks! Heres 100 coins for your efforts.")
                    (`/Game/BluePrints/WB_UI.RemoveQuest` (`/Game/BluePrints/BP_GameMode.UI` _asbp_game_mode) (make `/Game/BluePrints/Quest` (`self.CurrentQuest`) self))
                    (set `self.CurrentQuest` null)
                    (`self.K2_DestroyActor` _helditem)
                    (else
                      (`TextBlock.SetText` _talktext (`KismetTextLibrary.Conv_StringToText` (`self.GetRandomElement` (`self.Dialogues`))) :!label _label_4))))
                (:`else`
                  (if (<= (`KismetMathLibrary.RandomFloat`) 0.1)
                    (bind _asbp_game_mode_2 (cast `/Game/BluePrints/BP_GameMode` (`GameplayStatics.GetGameMode`)))
                    (bind _output_get_3 (set `self.CurrentQuest` (`self.GetRandomQuestItem` (`/Game/BluePrints/BP_GameMode.QuestItems` _asbp_game_mode_2))))
                    (`TextBlock.SetText` _talktext (`KismetTextLibrary.Conv_StringToText` (`KismetStringLibrary.Concat_StrStr` "Could you bring me a " (defaults `Object` _output_get_3))))
                    (`/Game/BluePrints/WB_UI.AddQuest` (`/Game/BluePrints/BP_GameMode.UI` _asbp_game_mode_2) (make `/Game/BluePrints/Quest` _output_get_3 self))
                    (else
                      (goto _label_4)))))
              (else
                ;[1 1 1] Shop
                (bind _shopui_2 (`self.ShopUI` :!label _label_5)
                  (:`then`
                    (`Widget.SetVisibility` _shopui_2 "Visible")
                    (`/Game/BluePrints/WB_NPCShop.UpdateNpcShop` (stale _returnvalue_3) _shopitems))
                  (:`else`
                    (bind _returnvalue_3 (`|CreateWidget` "/Game/BluePrints/WB_NPCShop.WB_NPCShop_C"))
                    (`/Game/BluePrints/WB_NPCShop.UpdateNpcShop` _returnvalue_3 _shopitems)
                    (bind _output_get_4 (set `self.ShopUI` _returnvalue_3))))
                (`UserWidget.AddToViewport` _output_get_4 0)
                (`UserWidget.AddToViewport` (`self.ShopUI`) 0)
                (`WidgetBlueprintLibrary.SetInputMode_GameAndUIEx` _returnvalue _output_get_4 "DoNotLock" false)
                (set `PlayerController.bShowMouseCursor` true _returnvalue))))
          (:`else`
            (goto _label_5)))
        (else
          (goto _label_3))))))

(fn `UserConstructionScript`)