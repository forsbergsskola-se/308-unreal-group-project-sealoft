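; Bed actor that loads the KaleLevel level instance when the player is inside a box area.
; BeginPlay loads the "save" slot and casts it to BP_SaveGame without using the result, or creates and saves a new one if absent.
; Tick runs a box overlap at fixed world coordinates for BP_Player, calling Save on every overlapping frame.
; Despite its name, Save only loads the level instance and writes no save data.
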(event `self.ReceiveBeginPlay`
  (bind _returnvalue (`GameplayStatics.DoesSaveGameExist` "save"))
  (if _returnvalue
    (bind _returnvalue_2 (`GameplayStatics.LoadGameFromSlot` "save"))
    (cast `/Game/BluePrints/BP_SaveGame` _returnvalue_2)
    (else
      (bind _returnvalue_3 (`GameplayStatics.CreateSaveGameObject` "/Game/BluePrints/BP_SaveGame.BP_SaveGame_C"))
      (`GameplayStatics.SaveGameToSlot` _returnvalue_3 "save"))))

(event `self.ReceiveTick`
  (params (DeltaSeconds :type "Float (single-precision)"))
  (bind (_outactors _returnvalue) (`KismetSystemLibrary.BoxOverlapActors` :`BoxPos` (0.0 0.0 26.010487) :`BoxExtent` (232.111706 341.253952 114.427818) :`ActorClassFilter` "/Game/BluePrints/BP_Player.BP_Player_C"))
  (if _returnvalue
    (`self.Save`)))

(fn `Save`
  (`LevelStreamingDynamic.LoadLevelInstance` "KaleLevel" (0.0 0.0 0.0) (struct) "" null))

(fn `UserConstructionScript`)