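; BP_Parkingspot is an interactable parking spot actor that gives the player a fresh moped.
; On interaction it prints a debug message and reads the current moped reference from BP_GameMode.
; It destroys any existing moped, spawns a new Moped_v2_Pawn at its MopedSpawnPoint location, and stores it back in the game mode, so only one tracked moped exists at a time.
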(event `/Game/BluePrints/IInteractable.On Interacted With`
  (params (Player :type "/Game/BluePrints/BP_Player Object Reference"))
  (`KismetSystemLibrary.PrintString` "Interacted with parkingspot")
  (bind _asbp_game_mode (cast `/Game/BluePrints/BP_GameMode` (`GameplayStatics.GetGameMode`)))
  (bind _currentmoped (`/Game/BluePrints/BP_GameMode.CurrentMoped` _asbp_game_mode))
  (`/Engine/EditorBlueprintResources/StandardMacros.IsValid` _currentmoped
    (:`Is Valid`
      (`self.K2_DestroyActor` _currentmoped))
    (:`Is Not Valid`
      _))
  (bind _returnvalue (`|SpawnActorFromClass` "/Game/VehicleTemplate/Blueprints/Moped_v2/Moped_v2_Pawn.Moped_v2_Pawn_C" (`KismetMathLibrary.MakeTransform` (`SceneComponent.K2_GetComponentLocation` (`self.Moped Spawn Point`)) (`self.Spawn Transform Rotation`)) "Undefined" "MultiplyWithRoot" null null))
  (set `/Game/BluePrints/BP_GameMode.CurrentMoped` _returnvalue _asbp_game_mode))

(fn `UserConstructionScript`)